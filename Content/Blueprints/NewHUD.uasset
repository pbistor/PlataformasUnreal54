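; NewHUD is the HUD class that owns the in-game canvas and pause menu widgets.
; On BeginPlay it creates both, showing the canvas immediately and holding the pause menu until needed.
; It forwards life changes, save notices and timed text messages to the canvas.
; Pause toggles game pause, adding or removing the menu and switching input mode and mouse cursor to match.
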(event `self.ReceiveBeginPlay`
  (bind _returnvalue (`self.GetOwningPlayerController`))
  (bind _returnvalue_2 (`|CreateWidget` "/Game/WBP_Canvas.WBP_Canvas_C" _returnvalue))
  (bind _output_get (set `self.GameWidget` _returnvalue_2))
  (`UserWidget.AddToViewport` _output_get 0)
  (bind _returnvalue_3 (`|CreateWidget` "/Game/WBP_PauseMenu.WBP_PauseMenu_C" _returnvalue))
  (set `self.PauseMenu` _returnvalue_3))

(event `ShowSaveUI`
  (`/Game/WBP_Canvas.ShowSave` (`self.GameWidget`)))

(event `ShowTextInfo`
  (params (Text :type Text) (Time :type "Float (double-precision)"))
  (`/Game/WBP_Canvas.ShowText` (`self.GameWidget`) Text Time))

(fn `LifeChanged`
  (params (NewLife :type "Float (double-precision)"))
  (`/Game/WBP_Canvas.UpdateLife` (`self.GameWidget`) NewLife))

(fn `Pause`
  (bind _returnvalue (`self.GetOwningPlayerController`))
  (bind _pausemenu (`self.PauseMenu`))
  (if (`self.isPaused`)
    (`GameplayStatics.SetGamePaused` false)
    (`Widget.RemoveFromParent` (`self.PauseMenu`))
    (`WidgetBlueprintLibrary.SetInputMode_GameOnly` _returnvalue)
    (set `self.isPaused` false)
    (set `PlayerController.bShowMouseCursor` false _returnvalue)
    (else
      (`GameplayStatics.SetGamePaused` true)
      (`UserWidget.AddToViewport` _pausemenu 0)
      (`WidgetBlueprintLibrary.SetInputMode_UIOnlyEx` _returnvalue _pausemenu)
      (set `self.isPaused` true)
      (set `PlayerController.bShowMouseCursor` true _returnvalue))))

(fn `UserConstructionScript`)